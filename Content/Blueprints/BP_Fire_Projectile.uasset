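; Fire projectile that damages BPI_Stats actors it hits, skipping those with a matching tag.
; Tick copies the player's RangeDamage into Damage and TempDamage every frame.
; On hit it attaches to the struck actor, cuts Damage to a tenth, and destroys itself after a delay, lengthened for non-stat actors.
; The construction script tints the mesh materials through the Colour parameter.
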(event `self.ReceiveTick`
  (params (DeltaSeconds :type "Float (single-precision)"))
  (bind _output_get (set `self.Damage` (`BaseCharacter.RangeDamage` (cast `/Game/Blueprints/Characters/BP_BaseCharacter` (`GameplayStatics.GetPlayerPawn` 0) :!pure true))))
  (set `self.TempDamage` _output_get))

(event `self.ReceiveBeginPlay`)

(event `self.ReceiveHit`
  (params (MyComp :type "PrimitiveComponent Object Reference") (Other :type "Actor Object Reference") (OtherComp :type "PrimitiveComponent Object Reference") (bSelfMoved :type Boolean) (HitLocation :type "Vector Structure") (HitNormal :type "Vector Structure") (NormalImpulse :type "Vector Structure") (Hit :type "HitResult Structure (by ref)"))
  (bind _sphere (`self.Sphere`))
  (if (`KismetSystemLibrary.DoesImplementInterface` Other "/Game/Blueprints/Interfaces/BPI_Stats.BPI_Stats_C")
    (if (not (`self.ActorHasTag` Other (`self.Tag`)))
      (message `/Game/Blueprints/Interfaces/BPI_Stats.AffectHealth` Other (`self.Damage`))
      (`self.K2_AttachToActor` Other "None" "KeepWorld" "KeepWorld" "KeepWorld" :!label _label)
      (bind _output_get (set `self.Damage` (* (`self.TempDamage`) 0.1)))
      (`KismetSystemLibrary.Delay` (`self.Duration`))
      (else
        (`PrimitiveComponent.IgnoreActorWhenMoving` _sphere Other true)
        (`PrimitiveComponent.SetCollisionEnabled` _sphere "NoCollision")))
    (else
      (set `self.Duration` 5.0)
      (goto _label)))
  (`self.K2_DestroyActor`))

(fn `UserConstructionScript`
  (`MeshComponent.SetVectorParameterValueOnMaterials` (`self.StaticMesh`) "Colour" (`KismetMathLibrary.Conv_LinearColorToVector` (`self.Colour`))))