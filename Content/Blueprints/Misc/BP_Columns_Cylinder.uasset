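; BP_Columns_Cylinder is a decorative column actor with a coloured, animated crystal and a matching point light.
; The construction script applies the Colour variable to a dynamic material instance on the Crystal and to the PointLight.
; On BeginPlay, the RotateFloat timeline drives the crystal's yaw and adds its Float track to the current relative Z each update, so the height offset accumulates.
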(event `self.ReceiveBeginPlay`
  (bind _crystal (`self.Crystal`))
  (bind (_direction _rotate _float) (`Timeline|Rotate/Float`)
    (:`Update`
      (`SceneComponent.K2_SetRelativeLocationAndRotation` _crystal (`KismetMathLibrary.MakeVector` 0.0 0.0 (+ (.z (`SceneComponent.RelativeLocation` _crystal)) _float)) (`KismetMathLibrary.MakeRotator` 0.0 0.0 _rotate) false false))))

(fn `UserConstructionScript`
  (bind _colour (`self.Colour`))
  (bind _returnvalue (`PrimitiveComponent.CreateDynamicMaterialInstance` (`self.Crystal`) 0 null))
  (`MaterialInstanceDynamic.SetVectorParameterValue` _returnvalue "Colour" _colour)
  (`LightComponent.SetLightColor` (`self.PointLight`) _colour true))