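; BP_Columns_Spiral is a decorative spiral column with a rotating, tintable static mesh.
; The construction script creates a dynamic material on the mesh and sets its Colour parameter from OrbColour.
; On BeginPlay it spawns a scaled-down BP_AmbientLights actor above itself and plays the Rotate timeline, which drives the mesh's relative yaw.
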(event `self.ReceiveBeginPlay`
  (`|SpawnActorFromClass` "/Game/Blueprints/Misc/BP_AmbientLights.BP_AmbientLights_C" (`KismetMathLibrary.MakeTransform` (`KismetMathLibrary.MakeVector` (.x (`self.K2_GetActorLocation`)) (.y (`self.K2_GetActorLocation`)) (+ (.z (`self.K2_GetActorLocation`)) 300.0)) (struct) (0.25 0.25 0.25)) "Undefined" "OverrideRootScale" null null)
  (bind (_direction _rotate) (`Timeline|Rotate`)
    (:`Update`
      (`SceneComponent.K2_SetRelativeRotation` (`self.StaticMesh`) (`KismetMathLibrary.MakeRotator` 0.0 0.0 _rotate) false false))))

(fn `UserConstructionScript`
  (bind _returnvalue (`PrimitiveComponent.CreateDynamicMaterialInstance` (`self.StaticMesh`) 0 null))
  (`MaterialInstanceDynamic.SetVectorParameterValue` _returnvalue "Colour" (`self.OrbColour`)))