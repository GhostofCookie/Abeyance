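; BP_PuzzleArea is an overlap area that pulls the player camera back while active, presumably for puzzle sections.
; On begin overlap by any actor, it stores player pawn 0's spring arm length, extends it and disables the arm's collision test.
; The one-shot FInterpTo uses a large delta time, so the change is instant.
; End overlap restores the saved length and re-enables the collision test.
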(event `self.ReceiveActorBeginOverlap`
  (params (OtherActor :type "Actor Object Reference"))
  (bind _asbp_base_character (cast `/Game/Blueprints/Characters/BP_BaseCharacter` (`GameplayStatics.GetPlayerPawn` 0)))
  (bind _springarm (`/Game/Blueprints/Characters/BP_BaseCharacter.SpringArm` _asbp_base_character))
  (bind _targetarmlength (`SpringArmComponent.TargetArmLength` _springarm))
  (set `self.OriginalArmLength` _targetarmlength)
  (set `SpringArmComponent.TargetArmLength` (`KismetMathLibrary.FInterpTo` _targetarmlength 1000.0 100.0 1.0) _springarm)
  (set `SpringArmComponent.bDoCollisionTest` false _springarm))

(event `self.ReceiveActorEndOverlap`
  (params (OtherActor :type "Actor Object Reference"))
  (bind _asbp_base_character (cast `/Game/Blueprints/Characters/BP_BaseCharacter` (`GameplayStatics.GetPlayerPawn` 0)))
  (bind _springarm (`/Game/Blueprints/Characters/BP_BaseCharacter.SpringArm` _asbp_base_character))
  (set `SpringArmComponent.TargetArmLength` (`self.OriginalArmLength`) _springarm)
  (set `SpringArmComponent.bDoCollisionTest` true _springarm))

(fn `UserConstructionScript`)