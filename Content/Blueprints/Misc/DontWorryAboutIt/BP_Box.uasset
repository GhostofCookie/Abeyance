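; BP_Box is a one-shot animated box that responds to a Collect event while the player pawn overlaps it.
; A DoOnce gate starts the Box_Anim skeletal animation, plays an attenuated sound attached to the mesh and reveals a material billboard.
; After a fixed delay of about twenty seconds, it plays Box_Anim1 and hides the billboard again.
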(event `/Game/Blueprints/Interfaces/BPI_Interact.Collect`
  (if (`self.IsOverlappingActor` (`GameplayStatics.GetPlayerPawn` 0))
    (`/Engine/EditorBlueprintResources/StandardMacros.DoOnce` false
      (:`Completed`
        (`SkeletalMeshComponent.PlayAnimation` (`self.SkeletalMesh`) "/Game/Blueprints/Misc/DontWorryAboutIt/Box_Anim.Box_Anim" false)
        (`GameplayStatics.SpawnSoundAttached` "/Game/Blueprints/Misc/DontWorryAboutIt/Box.Box" (`self.SkeletalMesh`) "None" (0.0 0.0 0.0) (struct) "KeepRelativeOffset" false 0.25 1.0 0.0 "/Game/Blueprints/Misc/DontWorryAboutIt/SA_Box.SA_Box")
        (`SceneComponent.SetVisibility` (`self.MaterialBillboard`) true false)
        (`KismetSystemLibrary.Delay` 20.19)
        (`SkeletalMeshComponent.PlayAnimation` (`self.SkeletalMesh`) "/Game/Blueprints/Misc/DontWorryAboutIt/Box_Anim1.Box_Anim1" false)
        (`SceneComponent.SetVisibility` (`self.MaterialBillboard`) false false)))))

(fn `UserConstructionScript`)