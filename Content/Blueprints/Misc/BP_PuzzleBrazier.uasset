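; BP_PuzzleBrazier is a puzzle brazier that can be toggled lit or unlit, spawning a coloured BP_AmbientLights actor when lit.
; Overlap shows or hides a W_PressButton prompt, whose icon Tick refreshes for gamepad or keyboard.
; Collect marks the widget pressed and flip-flops Activated.
; Once the widget reports Complete, Tick spawns the light through a DoOnce, or destroys it and resets the gate when deactivated.
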(event `self.ReceiveTick`
  (params (DeltaSeconds :type "Float (single-precision)"))
  (bind _lightref (`self.LightRef`))
  (`self.SetWidget`)
  (if (`/Game/UI/W_PressButton.Complete` (`self.WidgetRef`))
    (if (`self.Activated?`)
      (`/Engine/EditorBlueprintResources/StandardMacros.DoOnce` false :!label _label
        (:`Completed`
          (`self.Spawn Light`)))
      (else
        (`/Engine/EditorBlueprintResources/StandardMacros.IsValid` _lightref
          (:`Is Valid`
            (`self.K2_DestroyActor` _lightref)
            (goto _label :!via `Reset`)))))))

(event `self.ReceiveBeginPlay`
  (bind _asbp_base_character (cast `/Game/Blueprints/Characters/BP_BaseCharacter` (`GameplayStatics.GetPlayerPawn` 0)))
  (set `self.PlayerRef` _asbp_base_character))

(event `self.ReceiveActorBeginOverlap`
  (params (OtherActor :type "Actor Object Reference"))
  (`SceneComponent.SetVisibility` (`self.Widget`) true false))

(event `/Game/Blueprints/Interfaces/BPI_Interact.Collect`
  (set `/Game/UI/W_PressButton.IsPressed?` true (`self.WidgetRef`))
  (`/Engine/EditorBlueprintResources/StandardMacros.FlipFlop`
    (:`A`
      (set `self.Activated?` true))
    (:`B`
      (set `self.Activated?` false))))

(event `self.ReceiveActorEndOverlap`
  (params (OtherActor :type "Actor Object Reference"))
  (`SceneComponent.SetVisibility` (`self.Widget`) false false))

(fn `SetWidget`
  (bind _button (`/Game/UI/W_PressButton.Button` (`self.WidgetRef`)))
  (bind _asw_press_button (cast `/Game/UI/W_PressButton` (`WidgetComponent.GetUserWidgetObject` (`self.Widget`))))
  (set `self.WidgetRef` _asw_press_button)
  (bind _returnvalue (`GamepadDetection.IsGamePadConnected`))
  (if _returnvalue
    (`Image.SetBrushFromTexture` _button "/Game/Textures/GamepadButtons/Xbox/Xbox_RightStick.Xbox_RightStick" false)
    (else
      (`Image.SetBrushFromTexture` _button "/Game/Textures/GamepadButtons/PC/PC_Shift.PC_Shift" false))))

(fn `Spawn Light`
  (bind _returnvalue (`|SpawnActorFromClass` "/Game/Blueprints/Misc/BP_AmbientLights.BP_AmbientLights_C" (`KismetMathLibrary.MakeTransform` (`SceneComponent.K2_GetComponentLocation` (`self.LightSpawn`)) (struct) (0.5 0.5 0.5)) "Undefined" "OverrideRootScale" null null))
  (bind _output_get (set `self.LightRef` _returnvalue))
  (set `/Game/Blueprints/Misc/BP_AmbientLights.Colour` (`self.Colour`) _output_get))

(fn `UserConstructionScript`)