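; Level loader trigger actor that streams in a randomly chosen room sub-level when overlapped, then unloads it and destroys itself when the overlap ends.
; It picks one of four room entries, creates a streaming level instance with a random-number name suffix, and places it at the actor's rotation and XY-offset location.
; The construction script scales the trigger box from exposed X and Y values.
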(event `self.Trigger.OnComponentBeginOverlap`
  (params (OverlappedComponent :type "PrimitiveComponent Object Reference") (OtherActor :type "Actor Object Reference") (OtherComp :type "PrimitiveComponent Object Reference") (OtherBodyIndex :type Integer) (bFromSweep :type Boolean) (SweepResult :type "HitResult Structure (by ref)"))
  (bind _loadlevel (`self.LoadLevel`))
  (bind _loadlevel_2 (`self.LoadLevel`))
  ;[0.5354 0 1] Creates unique instances of the sub-levels, and loads them randomly in front of and behind the player
  (`/Engine/EditorBlueprintResources/StandardMacros.IsValid` _loadlevel
    (:`Is Valid`
      (set `LevelStreaming.bShouldBeLoaded` false _loadlevel)
      (set `LevelStreaming.bShouldBeVisible` false _loadlevel))
    (:`Is Not Valid`
      _))
  (bind _level_to_load (`self.RandomizeRoom` 0 3))
  (`self.LoadLevelInstance` _level_to_load (`self.K2_GetActorLocation`) (`self.X Offset`) (`self.Y Offset`))
  (set `LevelStreaming.bShouldBeLoaded` true _loadlevel_2)
  (set `LevelStreaming.bShouldBeVisible` true _loadlevel_2))

(event `self.Trigger.OnComponentEndOverlap`
  (params (OverlappedComponent :type "PrimitiveComponent Object Reference") (OtherActor :type "Actor Object Reference") (OtherComp :type "PrimitiveComponent Object Reference") (OtherBodyIndex :type Integer))
  (bind _loadlevel (`self.LoadLevel`))
  (`/Engine/EditorBlueprintResources/StandardMacros.IsValid` _loadlevel
    (:`Is Valid`
      (set `LevelStreaming.bShouldBeLoaded` false _loadlevel)
      (set `LevelStreaming.bShouldBeVisible` false _loadlevel)
      (`self.K2_DestroyActor`))))

(fn `LoadLevelInstance`
  (params (LevelToLoad :type Name) (InVec :type "Vector Structure") (`X Offset` :type "Float (double-precision)") (`Y Offset` :type "Float (double-precision)"))
  (bind (_returnvalue_location _returnvalue_rotation) (`KismetMathLibrary.BreakTransform` (`KismetMathLibrary.MakeTransform` (`KismetMathLibrary.MakeVector` (+ (.x InVec) `X Offset`) (+ (.y InVec) `Y Offset`) (.z InVec)) (`self.K2_GetActorRotation`))))
  (bind _returnvalue (`LevelStreaming.CreateInstance` (`GameplayStatics.GetStreamingLevel` LevelToLoad) (`KismetStringLibrary.Concat_StrStr` (`KismetStringLibrary.Conv_NameToString` (`self.LevelToLoad`)) (`KismetStringLibrary.Conv_IntToString` (`KismetMathLibrary.RandomInteger` 100)))))
  (`/Engine/EditorBlueprintResources/StandardMacros.IsValid` _returnvalue
    (:`Is Valid`
      (set `LevelStreaming.LevelTransform` (`KismetMathLibrary.MakeTransform` _returnvalue_location _returnvalue_rotation) _returnvalue)
      (set `self.LoadLevel` _returnvalue))))

(fn `RandomizeRoom`
  (params (Min :type Integer) (Max :type Integer))
  (returns (`Level To Load` :type Name))
  (bind _output_get (set `self.LevelToLoad` (`|GetArrayItem` (`.Rooms_0_16_57F06A2A4753C47D1DAFB5B9BE8081E8` (break `/Game/Blueprints/Structs/S_Rooms` (`self.Rooms`))) (`KismetMathLibrary.RandomIntegerInRange` Min Max))))
  (return _output_get))

(fn `UserConstructionScript`
  (`SceneComponent.SetWorldScale3D` (`self.Trigger`) (`KismetMathLibrary.MakeVector` (`self.TriggerX`) (`self.TriggerY`) 1.0)))