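; BP_Character_Effects is an unfinished tracker for a character's active ability effects.
; Construction sizes ActiveAbilityList and AbilitiesOnTick from the DT_Skills row count.
; Tick only loops over AbilitiesOnTick without acting, and the reset and get functions are stubs.
; Disconnected graph logic would apply timed stat changes through AffectStatMessage, or swap to a fire projectile for the Fire ability, followed by a cooldown.
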(event `self.ReceiveTick`
  (params (DeltaSeconds :type "Float (single-precision)"))
  ;[1 1 1] check active list vs stored list, if different, update active effects. Else re-write ability_list with active abilities
  (for (_ _array_index) (`self.Abilities_On_Tick`)
    (if (== false false)
      _)))

(fn `Get_Active_Effects`
  ;[1 1 1] if effect is active, mark Abilities_On_Tick[abilityIndex] as 1 else 0
  (for _ (`self.Abilities_On_Tick`)
    _))

(fn `Reset_Active_Effects`)

(fn `UserConstructionScript`
  (locals (NewLocalVar_1 :type "/Game/UI/SkillTree/W_SkillTree Object Reference"))
  ;[1 1 1] construct array for active effects
  (bind _outrownames (`DataTableFunctionLibrary.GetDataTableRowNames` "/Game/UI/SkillTree/DT_Skills.DT_Skills"))
  (bind _output_get (set `self.Effects_Size` (`KismetArrayLibrary.Array_Length` _outrownames)))
  (`KismetArrayLibrary.Array_Resize` (`self.Active_Ability_List`) _output_get)
  (`KismetArrayLibrary.Array_Resize` (`self.Abilities_On_Tick`) _output_get))