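; Player controller that handles the pause menu, companion menu and brazier collection input.
; OpenMenu toggles a pause widget created at BeginPlay, switching cursor, input mode and move/look blocking, with force feedback.
; CompanionMenu messages the first Companion found; Z or right-thumbstick press messages overlapping puzzle braziers to collect.
; Tick converts held-key time into clamped ButtonHold progress and accumulates right-stick input into a bounded cursor position.
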(event `InputAction|OpenMenu`
  (params (Key :type "Key Structure"))
  (bind _pausemenuref (`self.PauseMenuRef`))
  (:`Pressed`
    (bind _returnvalue (`GamepadDetection.IsGamePadConnected`))
    (if _returnvalue
      _
      (else
        _))
    (if (`/Game/UI/W_Pause.Closed?` _pausemenuref)
      (set `self.bShowMouseCursor` true)
      (set `/Game/UI/W_Pause.Closed?` false _pausemenuref)
      (`UserWidget.AddToViewport` _pausemenuref 0)
      (`WidgetBlueprintLibrary.SetInputMode_GameAndUIEx` self)
      (`self.SetIgnoreLookInput` self true)
      (`self.SetIgnoreMoveInput` self true)
      (else
        (set `self.bShowMouseCursor` false)
        (set `/Game/UI/W_Pause.Closed?` true _pausemenuref)
        (`Widget.RemoveFromParent` _pausemenuref)
        (`WidgetBlueprintLibrary.SetInputMode_GameOnly` self)
        (`self.SetIgnoreLookInput` false)
        (`self.SetIgnoreMoveInput` false)))
    (`self.PlayDynamicForceFeedback` 10.0 0.2)))

(event `self.ReceiveBeginPlay`
  (bind _outactors (`GameplayStatics.GetAllActorsOfClass` "/Game/Blueprints/Characters/Companion/Companion.Companion_C"))
  (set `self.CompanionRef` (`|GetArrayItem` _outactors))
  (set `self.bShowMouseCursor` false)
  (`WidgetBlueprintLibrary.SetInputMode_GameOnly` self)
  (bind _returnvalue (`|CreateWidget` "/Game/UI/W_Pause.W_Pause_C"))
  (set `self.PauseMenuRef` _returnvalue))

(event `self.ReceiveTick`
  (params (DeltaSeconds :type "Float (single-precision)"))
  (bind (_stickx _sticky) (`self.GetInputAnalogStickState` "CAS_RightStick"))
  (`self.HoldKey` (`self.CurrentKey`))
  (set `self.CursorX` (`KismetMathLibrary.FClamp` (+ (`self.CursorX`) (* _stickx 50.0)) -750.0 750.0))
  (set `self.CursorY` (`KismetMathLibrary.FClamp` (+ (* _sticky 50.0) (`self.CursorY`)) -500.0 500.0))
  (set `self.CursorPosition` (`KismetMathLibrary.MakeVector2D` (`self.CursorX`) (`self.CursorY`))))

(event `MainMenu`
  (bind _output_get (set `self.MenuNavigation` (`.StickY` (`self.GetInputAnalogStickState` "CAS_LeftStick"))))
  (`KismetSystemLibrary.PrintString` (`KismetStringLibrary.Conv_DoubleToString` _output_get)))

(event `InputAction|CompanionMenu`
  (params (Key :type "Key Structure"))
  ;[0 1 0.7518] Open menu from Companion
  (:`Pressed`
    (set `self.CurrentKey` Key)
    (set `self.IsHolding?` true)
    (if (`self.IsHolding?`)
      (message `/Game/Blueprints/Interfaces/BPI_Interact.CompanionMenu` (`self.CompanionRef`))))
  (:`Released`
    (set `self.IsHolding?` false)))

(event `Key|Gamepad_RightThumbstick`
  (params (Key :type "Key Structure"))
  (:`Pressed`
    (set `self.CurrentKey` Key)
    (set `self.IsHolding?` true)
    (if (`self.IsHolding?`) :!label _label
      (for _array_element (`self.GetOverlappingActors` (`GameplayStatics.GetPlayerPawn` 0) "/Game/Blueprints/Misc/BP_PuzzleBrazier.BP_PuzzleBrazier_C")
        (message `/Game/Blueprints/Interfaces/BPI_Interact.Collect` _array_element))))
  (:`Released`
    (set `self.IsHolding?` false)))

(event `Key|Z`
  (params (Key :type "Key Structure"))
  (:`Pressed`
    (set `self.CurrentKey` Key)
    (set `self.IsHolding?` true)
    (goto _label))
  (:`Released`
    (set `self.IsHolding?` false)))

(fn `HoldKey`
  (params (Key :type "Key Structure"))
  (if (`self.IsHolding?`)
    (set `self.ButtonHold` (`KismetMathLibrary.FClamp` (/ (`self.GetInputKeyTimeDown` Key) 1.0)))
    (else
      (set `self.ButtonHold` 0.0))))

(fn `UserConstructionScript`)