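; Collectible artifact that, when its Collect event is called, ends the level and destroys itself.
; LevelEnd plays an explosion sound, spawns a BP_PortalDoor_Local at the DoorSpawn offset with the artifact's PortalID, and starts a camera fade.
; Each tick, its prompt widget yaws toward the camera, shows only near the player, and swaps its button icon between gamepad and keyboard.
; An unconnected branch for removing all portals never runs.
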(event `self.ReceiveTick`
  (params (DeltaSeconds :type "Float (single-precision)"))
  (`self.ActivateText` (`self.Widget`) 1.0)
  (`self.SetWidget`))

(event `/Game/Blueprints/Interfaces/BPI_Interact.Collect`
  (`self.LevelEnd`)
  (`self.K2_DestroyActor`))

(event `LevelEnd`
  (`GameplayStatics.PlaySoundAtLocation` "/Game/StarterContent/Audio/Explosion02.Explosion02")
  (bind _returnvalue (`|SpawnActorFromClass` "/Game/Blueprints/Portals/BP_PortalDoor_Local.BP_PortalDoor_Local_C" (`KismetMathLibrary.MakeTransform` (+ (`self.DoorSpawn`) (`self.K2_GetActorLocation`)) (`self.K2_GetActorRotation`)) "Undefined" "OverrideRootScale" null null))
  (set `/Game/Blueprints/Portals/BP_PortalDoorBase.PortalID` (`self.PortalID`) _returnvalue)
  (`PlayerCameraManager.StartCameraFade` :`self` (`GameplayStatics.GetPlayerCameraManager` 0) :`FromAlpha` 1.0 :`Duration` 5.0 :`bShouldFadeAudio` true :`bHoldWhenFinished` true))

(fn `ActivateText`
  (params (Component :type "SceneComponent Object Reference") (MinDistance :type "Float (double-precision)"))
  (`self.RotateToCamera` Component)
  (bind _returnvalue (`self.DistanceToPlayer` MinDistance))
  (if _returnvalue
    (`SceneComponent.SetVisibility` Component true false)
    (else
      (`SceneComponent.SetVisibility` Component false false))))

(fn `DistanceToPlayer`
  (params (MinDistance :type "Float (double-precision)"))
  (returns (ReturnValue :type Boolean))
  (return (<= (`self.GetDistanceTo` (`GameplayStatics.GetPlayerPawn` 0) self) (* MinDistance 200.0))))

(fn `RotateToCamera`
  (params (Component :type "SceneComponent Object Reference"))
  (`SceneComponent.K2_SetWorldRotation` Component (`KismetMathLibrary.Conv_VectorToRotator` (`KismetMathLibrary.GreaterGreater_VectorRotator` (`KismetMathLibrary.Normal` (* (- (`PlayerCameraManager.GetCameraLocation` (`GameplayStatics.GetPlayerCameraManager` 0)) (`SceneComponent.K2_GetComponentLocation` Component)) (1.0 1.0 0.0))))) false false))

(fn `SetWidget`
  (bind _button (`/Game/UI/W_PressButton.Button` (`self.WidgetRef`)))
  (bind _asw_press_button (cast `/Game/UI/W_PressButton` (`WidgetComponent.GetUserWidgetObject` (`self.Widget`))))
  (set `self.WidgetRef` _asw_press_button)
  (bind _returnvalue (`GamepadDetection.IsGamePadConnected`))
  (if _returnvalue
    (`Image.SetBrushFromTexture` _button "/Game/Textures/GamepadButtons/Xbox/Xbox_RightStick.Xbox_RightStick" false)
    (else
      (`Image.SetBrushFromTexture` _button "/Game/Textures/GamepadButtons/PC/PC_Shift.PC_Shift" false))))

(fn `UserConstructionScript`)