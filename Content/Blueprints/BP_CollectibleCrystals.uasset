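; Collectible crystal cluster actor holding three crystal components that are harvested one at a time.
; Each Collect call destroys the first still-valid crystal in the order 1, 3, 2 and sets Collected true, or false when none remain.
; The construction script gives each crystal a dynamic material instance and tints its Colour parameter a translucent blue.
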(event `/Game/Blueprints/Interfaces/BPI_Interact.Collect`
  (bind _crystal1 (`self.Crystal1`))
  (bind _crystal2 (`self.Crystal2`))
  (bind _crystal3 (`self.Crystal3`))
  (`/Engine/EditorBlueprintResources/StandardMacros.IsValid` _crystal1
    (:`Is Valid`
      (`ActorComponent.K2_DestroyComponent` _crystal1)
      (set `self.Collected?` true))
    (:`Is Not Valid`
      (`/Engine/EditorBlueprintResources/StandardMacros.IsValid` _crystal3
        (:`Is Valid`
          (`ActorComponent.K2_DestroyComponent` _crystal3)
          (set `self.Collected?` true))
        (:`Is Not Valid`
          (`/Engine/EditorBlueprintResources/StandardMacros.IsValid` _crystal2
            (:`Is Valid`
              (`ActorComponent.K2_DestroyComponent` _crystal2)
              (set `self.Collected?` true))
            (:`Is Not Valid`
              (set `self.Collected?` false))))))))

(fn `UserConstructionScript`
  (for _array_element (`|MakeArray` (`self.Crystal1`) (`self.Crystal2`) (`self.Crystal3`))
    (bind _returnvalue (`PrimitiveComponent.CreateDynamicMaterialInstance` _array_element 0 null))
    (`MaterialInstanceDynamic.SetVectorParameterValue` _returnvalue "Colour" (struct :`G` 0.142757 :`B` 0.932292 :`A` 0.634))))