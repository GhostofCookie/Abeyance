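; Door spawner actor that spawns a BP_LevelLoader relative to its own transform when play begins.
; SpawnLevelFromDoor adds an X/Y/Z offset to the location and keeps the rotation and scale, though BeginPlay passes no offset.
; A yaw check against 89 degrees splits BeginPlay into two identical branches, each clearing CanLevelSpawn after spawning.
; The outer condition is hardwired true, so CanLevelSpawn never gates the spawn.
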(event `self.ReceiveBeginPlay`
  (bind _returnvalue (`self.GetTransform`))
  (if true
    (if (>= (.yaw (.rotation _returnvalue)) 89.0)
      (`self.SpawnLevelFromDoor` _returnvalue)
      (set `self.CanLevelSpawn?` false)
      (else
        (`self.SpawnLevelFromDoor` _returnvalue)
        (set `self.CanLevelSpawn?` false)))))

(fn `SpawnLevelFromDoor`
  (params (InTransform :type "Transform Structure (by ref)") (X :type "Float (double-precision)") (Y :type "Float (double-precision)") (Z :type "Float (double-precision)"))
  (`|SpawnActorFromClass` "/Game/Blueprints/BP_LevelLoader.BP_LevelLoader_C" (`KismetMathLibrary.MakeTransform` (+ (.location InTransform) (`KismetMathLibrary.MakeVector` X Y Z)) (.rotation InTransform) (.scale InTransform)) "Undefined" "OverrideRootScale" null null))

(fn `UserConstructionScript`)