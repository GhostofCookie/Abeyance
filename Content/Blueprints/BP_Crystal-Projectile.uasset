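; BP_Crystal-Projectile is a coloured crystal projectile that damages what it overlaps.
; The construction script applies its Colour to the mesh materials' Colour parameter and to its point light.
; On overlap, it sends Damage through an interface message to implementers lacking its Tag, then destroys itself.
; It ignores implementers carrying that Tag, and is destroyed without dealing damage by actors lacking the interface.
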(event `self.ReceiveActorBeginOverlap`
  (params (OtherActor :type "Actor Object Reference"))
  (if (`KismetSystemLibrary.DoesImplementInterface` OtherActor)
    (if (not (`self.ActorHasTag` OtherActor (`self.Tag`)))
      (message `/Game/Blueprints/Interfaces/BPI_Stats.AffectHealth` OtherActor (`self.Damage`))
      (`self.K2_DestroyActor` :!label _label))
    (else
      (goto _label))))

(fn `UserConstructionScript`
  (bind _colour (`self.Colour`))
  (`MeshComponent.SetVectorParameterValueOnMaterials` (`self.StaticMesh`) "Colour" (`KismetMathLibrary.Conv_LinearColorToVector` _colour))
  (`LightComponent.SetLightColor` (`self.PointLight`) _colour true))