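; BP_PortalDoor1 is one end of a portal pair, teleporting overlapping actors to its partner BP_PortalDoor2 and destroying itself when overlap ends.
; Tick finds the partner and moves its PortalView to the player camera's position, offset between doors, with matching rotation and clip-plane base at the partner.
; Teleporting flags the partner to block bounce-back, clearing after two seconds, and aligns player control rotation.
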(event `self.ReceiveBeginPlay`)

(event `self.Box.OnComponentBeginOverlap`
  (params (OverlappedComponent :type "PrimitiveComponent Object Reference") (OtherActor :type "Actor Object Reference") (OtherComp :type "PrimitiveComponent Object Reference") (OtherBodyIndex :type Integer) (bFromSweep :type Boolean) (SweepResult :type "HitResult Structure (by ref)"))
  (`self.PortalTeleport` OtherActor (`self.PortalClass`)))

(event `PortalTeleport`
  (params (Actor :type "Actor Object Reference") (ActorClass :type "Actor Class Reference"))
  (if (`self.IsTeleporting`)
    (`KismetSystemLibrary.Delay` 2.0)
    (set `self.IsTeleporting` false)
    (set `self.Teleported` true)
    (else
      (`self.TeleportToPortal` Actor ActorClass)
      (set `self.Teleported` true))))

(event `self.Box.OnComponentEndOverlap`
  (params (OverlappedComponent :type "PrimitiveComponent Object Reference") (OtherActor :type "Actor Object Reference") (OtherComp :type "PrimitiveComponent Object Reference") (OtherBodyIndex :type Integer))
  (`self.K2_DestroyActor`))

(event `self.ReceiveTick`
  (params (DeltaSeconds :type "Float (single-precision)"))
  (bind _outactors (`GameplayStatics.GetAllActorsOfClass` (`self.PortalClass`)))
  (bind _asbp_portal_door_2 (cast `/Game/Blueprints/Portals/BP_PortalDoor2` (`|GetArrayItem` _outactors)))
  (`/Engine/EditorBlueprintResources/StandardMacros.IsValid` _asbp_portal_door_2
    (:`Is Valid`
      (set `self.TargetPortal` _asbp_portal_door_2)
      (`self.RenderPortal`))))

(fn `RenderPortal`
  (bind _targetportal (`self.TargetPortal`))
  (bind _returnvalue (`self.K2_GetActorLocation` _targetportal))
  (bind _portalview (`/Game/Blueprints/Portals/BP_PortalDoor2.PortalView` _targetportal))
  (bind _transformcomponent (`PlayerCameraManager.TransformComponent` (`PlayerController.PlayerCameraManager` (`GameplayStatics.GetPlayerController` 0))))
  (`/Engine/EditorBlueprintResources/StandardMacros.IsValid` _targetportal
    (:`Is Valid`
      (`SceneComponent.K2_SetWorldLocationAndRotation` _portalview (+ (- _returnvalue (`self.K2_GetActorLocation`)) (`SceneComponent.K2_GetComponentLocation` _transformcomponent)) (`SceneComponent.K2_GetComponentRotation` _transformcomponent) false false)
      (set `SceneCaptureComponent2D.ClipPlaneBase` _returnvalue _portalview))))

(fn `TeleportToPortal`
  (params (Actor :type "Actor Object Reference") (ActorClass :type "Actor Class Reference"))
  (bind _targetportal (`self.TargetPortal`))
  (bind _returnvalue (`self.K2_GetActorRotation` _targetportal))
  (`/Engine/EditorBlueprintResources/StandardMacros.IsValid` _targetportal
    (:`Is Valid`
      (set `/Game/Blueprints/Portals/BP_PortalDoor2.IsTeleporting` true _targetportal)
      (`self.K2_TeleportTo` Actor (`self.K2_GetActorLocation` _targetportal) _returnvalue)
      (`Controller.SetControlRotation` (`Pawn.GetController` (`GameplayStatics.GetPlayerCharacter` 0)) _returnvalue))))

(fn `UserConstructionScript`)