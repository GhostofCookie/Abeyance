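; BP_PortalDoor2 is a portal door that teleports overlapping actors to a linked BP_PortalDoor and drives that portal's view.
; Tick finds the target by PortalID, then moves its PortalView capture with the player camera's offset and rotation, setting a clip plane.
; Box overlap teleports the actor and flags both portals to prevent bouncing, clearing after a delay on re-entry.
; Ending overlap destroys this door; render-target creation never runs.
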(event `self.ReceiveBeginPlay`)

(event `self.Box.OnComponentBeginOverlap`
  (params (OverlappedComponent :type "PrimitiveComponent Object Reference") (OtherActor :type "Actor Object Reference") (OtherComp :type "PrimitiveComponent Object Reference") (OtherBodyIndex :type Integer) (bFromSweep :type Boolean) (SweepResult :type "HitResult Structure (by ref)"))
  (`self.PortalTeleport` OtherActor))

(event `PortalTeleport`
  (params (Actor :type "Actor Object Reference"))
  (if (`self.IsTeleporting`)
    (`KismetSystemLibrary.Delay` 2.0)
    (set `self.IsTeleporting` false)
    (set `self.Teleported` false)
    (else
      (bind _teleported_ (`self.TeleportToPortal` Actor))
      (set `self.IsTeleporting` true)
      (set `self.Teleported` _teleported_))))

(event `self.Box.OnComponentEndOverlap`
  (params (OverlappedComponent :type "PrimitiveComponent Object Reference") (OtherActor :type "Actor Object Reference") (OtherComp :type "PrimitiveComponent Object Reference") (OtherBodyIndex :type Integer))
  (if true
    (`self.K2_DestroyActor`)))

(event `self.ReceiveTick`
  (params (DeltaSeconds :type "Float (single-precision)"))
  ;[1 1 1] Search for a portal to teleport to
  (`/Engine/EditorBlueprintResources/StandardMacros.IsValid` (`self.TargetPortal`)
    (:`Is Valid`
      (`self.RenderPortal`))
    (:`Is Not Valid`
      (bind _outactors (`GameplayStatics.GetAllActorsOfClass` (`self.PortalClass`)))
      (bind _asbp_portal_door (cast `/Game/Blueprints/Portals/BP_PortalDoor` (`|GetArrayItem` _outactors (`self.PortalID`))))
      (`/Engine/EditorBlueprintResources/StandardMacros.IsValid` _asbp_portal_door
        (:`Is Valid`
          (set `self.TargetPortal` _asbp_portal_door))))))

(event `self.Trigger.OnComponentBeginOverlap`
  (params (OverlappedComponent :type "PrimitiveComponent Object Reference") (OtherActor :type "Actor Object Reference") (OtherComp :type "PrimitiveComponent Object Reference") (OtherBodyIndex :type Integer) (bFromSweep :type Boolean) (SweepResult :type "HitResult Structure (by ref)")))

(fn `RenderPortal`
  (bind _returnvalue_x (`KismetMathLibrary.BreakVector` (`self.K2_GetActorLocation`)))
  (bind _targetportal (`self.TargetPortal`))
  (bind _returnvalue (`self.K2_GetActorLocation` _targetportal))
  (bind (_returnvalue_x_2 _returnvalue_y _returnvalue_z) (`KismetMathLibrary.BreakVector` (`self.K2_GetActorLocation` (`self.TargetPortal`))))
  (bind _portalview (`/Game/Blueprints/Portals/BP_PortalDoor.PortalView` _targetportal))
  (bind _transformcomponent (`PlayerCameraManager.TransformComponent` (`PlayerController.PlayerCameraManager` (`GameplayStatics.GetPlayerController` 0))))
  (`/Engine/EditorBlueprintResources/StandardMacros.IsValid` _targetportal
    (:`Is Valid`
      (`SceneComponent.K2_SetWorldLocationAndRotation` _portalview (+ (- _returnvalue (`self.K2_GetActorLocation`)) (`SceneComponent.K2_GetComponentLocation` _transformcomponent)) (`SceneComponent.K2_GetComponentRotation` _transformcomponent) false false)
      (set `SceneCaptureComponent2D.ClipPlaneBase` _returnvalue _portalview)
      (set `SceneCaptureComponent2D.ClipPlaneNormal` (`KismetMathLibrary.MakeVector` _returnvalue_x _returnvalue_y _returnvalue_z) _portalview))))

(fn `TeleportToPortal`
  (params (Actor :type "Actor Object Reference"))
  (returns (`Teleported?` :type Boolean))
  (bind _targetportal (`self.TargetPortal`))
  (`/Engine/EditorBlueprintResources/StandardMacros.IsValid` _targetportal
    (:`Is Valid`
      (set `/Game/Blueprints/Portals/BP_PortalDoor.IsTeleporting` true _targetportal)
      (bind _returnvalue (`self.K2_TeleportTo` Actor (`self.K2_GetActorLocation` _targetportal) (`self.K2_GetActorRotation` _targetportal)))
      (return _returnvalue))))

(fn `UserConstructionScript`)