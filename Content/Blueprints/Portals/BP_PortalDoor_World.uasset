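; BP_PortalDoor_World is a portal door that removes itself once a character leaves it while teleporting is allowed.
; On BeginPlay it runs the parent logic, then sets PortalClass to BP_PortalDoor_World_2, presumably its counterpart door.
; When a BaseCharacter ends overlap with the Box and CanTeleport is true, the actor destroys itself.
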(event `self.ReceiveBeginPlay`
  (`parent.ReceiveBeginPlay`)
  (set `self.PortalClass` "/Game/Blueprints/Portals/BP_PortalDoor_World_2.BP_PortalDoor_World_2_C"))

(event `self.Box.OnComponentEndOverlap`
  (params (OverlappedComponent :type "PrimitiveComponent Object Reference") (OtherActor :type "Actor Object Reference") (OtherComp :type "PrimitiveComponent Object Reference") (OtherBodyIndex :type Integer))
  (bind _asbase_character (cast `BaseCharacter` OtherActor))
  (`/Engine/EditorBlueprintResources/StandardMacros.IsValid` _asbase_character
    (:`Is Valid`
      (if (`self.CanTeleport`)
        (`self.K2_DestroyActor`)))))

(fn `UserConstructionScript`
  (`parent.UserConstructionScript`))