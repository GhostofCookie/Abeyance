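; Base portal door that shows a live view through a partner portal matched by ID and teleports the player and companion there.
; Proximity, or a one-time activation where required, plays the opening timeline and enables teleporting.
; Each tick mirrors the player camera onto the partner's clip-planed scene capture, whose render target feeds the frame material.
; Non-local portals spawn a level loader and destroy themselves when the teleport box overlap ends.
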(event `self.ReceiveBeginPlay`
  (bind _asbp_base_character (cast `/Game/Blueprints/Characters/BP_BaseCharacter` (`GameplayStatics.GetPlayerCharacter` 0)))
  (set `self.CharacterRef` _asbp_base_character)
  (`PrimitiveComponent.SetCollisionEnabled` (`self.Box`) "NoCollision")
  (`PrimitiveComponent.SetCollisionEnabled` (`self.Trigger`) "NoCollision")
  (if (not (`self.IsLocal?`))
    (bind _returnvalue (`|SpawnActorFromClass` "/Game/Blueprints/BP_LevelLoader.BP_LevelLoader_C" (`self.GetTransform`) "Undefined" "OverrideRootScale" null null))
    (set `self.LoaderRef` _returnvalue))
  (bind _returnvalue_2 (`GameUserSettings.GetGameUserSettings`))
  (bind (_returnvalue_x _returnvalue_y) (break `IntPoint` (`GameUserSettings.GetDesktopResolution` _returnvalue_2)))
  (bind _returnvalue_3 (`KismetRenderingLibrary.CreateRenderTarget2D` _returnvalue_x _returnvalue_y))
  (bind _output_get (set `self.RenderTarget` _returnvalue_3))
  (set `SceneCaptureComponent2D.TextureTarget` _output_get (`self.PortalView`)))

(event `self.Box.OnComponentBeginOverlap`
  (params (OverlappedComponent :type "PrimitiveComponent Object Reference") (OtherActor :type "Actor Object Reference") (OtherComp :type "PrimitiveComponent Object Reference") (OtherBodyIndex :type Integer) (bFromSweep :type Boolean) (SweepResult :type "HitResult Structure (by ref)"))
  (bind _companionref (`/Game/Blueprints/Characters/BP_BaseCharacter.CompanionRef` (`self.CharacterRef`)))
  (if (`self.CanRender`)
    (`self.PortalTeleport` OtherActor)
    (`KismetSystemLibrary.Delay` 1.0)
    (`/Engine/EditorBlueprintResources/StandardMacros.IsValid` _companionref
      (:`Is Valid`
        (`self.K2_TeleportTo` _companionref (- (`self.K2_GetActorLocation` OtherActor) (`self.GetActorForwardVector` OtherActor)) (`self.K2_GetActorRotation` OtherActor))))))

(event `PortalTeleport`
  (params (Actor :type "Actor Object Reference"))
  (if (`self.IsTeleporting`)
    (set `self.CanTeleport` false)
    (set `self.CanRender` false)
    (`KismetSystemLibrary.Delay` 1.0)
    (set `self.IsTeleporting` false)
    (else
      (bind _teleported (`self.TeleportToPortal` Actor (`self.TargetPortal`)))
      (set `self.IsTeleporting` true)
      (set `self.CanTeleport` _teleported))))

(event `self.Box.OnComponentEndOverlap`
  (params (OverlappedComponent :type "PrimitiveComponent Object Reference") (OtherActor :type "Actor Object Reference") (OtherComp :type "PrimitiveComponent Object Reference") (OtherBodyIndex :type Integer))
  (if (not (`self.IsLocal?`))
    (`self.K2_DestroyActor`)))

(event `self.ReceiveTick`
  (params (DeltaSeconds :type "Float (single-precision)"))
  (bind _trigger (`self.Trigger`))
  (bind _targetportal (`self.TargetPortal`))
  (bind _loaderref (`self.LoaderRef`))
  ;[1 1 1] Search for a portal to teleport to
  (bind _outactors (`GameplayStatics.GetAllActorsWithTag` "LevelSize"))
  (bind _output (`|GetArrayItem` _outactors))
  (if (`KismetSystemLibrary.IsValid` _output)
    (`/Engine/EditorBlueprintResources/StandardMacros.IsValid` _loaderref
      (:`Is Valid`
        (bind _output_get (set `/Game/Blueprints/BP_LevelLoader.TriggerScale` (`self.GetActorScale3D` _output) _loaderref)))
      (:`Is Not Valid`
        _))
    (else
      (`KismetSystemLibrary.PrintString` "Nothing")))
  (`/Engine/EditorBlueprintResources/StandardMacros.IsValid` _targetportal
    (:`Is Valid`
      (if (`self.RequiresActivation?`)
        (`PrimitiveComponent.SetCollisionEnabled` _trigger "NoCollision")
        (if (`self.Activate`)
          (`self.RenderPortal` _targetportal))
        (else
          (`PrimitiveComponent.SetCollisionEnabled` _trigger "QueryOnly")
          (if (`self.CanRender`)
            (`self.RenderPortal` _targetportal)))))
    (:`Is Not Valid`
      (`self.SetTargetPortal`))))

(event `ActivatePortal`
  (bind _targetportal (`self.TargetPortal`))
  (bind _box (`self.Box`))
  ;[1 1 1] Activate portal permanently
  (`/Engine/EditorBlueprintResources/StandardMacros.DoOnce` false
    (:`Completed`
      (`self.SetTargetPortal`
        (:`Completed`
          (set `self.Activate` true)
          (`PrimitiveComponent.SetCollisionEnabled` (`self.Trigger`) "QueryOnly")
          (`/Engine/EditorBlueprintResources/StandardMacros.IsValid` (`self.TargetPortal`) :!label _label
            (:`Is Valid`
              (bind _returnvalue (`PrimitiveComponent.CreateDynamicMaterialInstance` (`self.Frame`) 1 "/Game/Materials/M_PortalEffect_2_Inst.M_PortalEffect_2_Inst"))
              (`MaterialInstanceDynamic.SetTextureParameterValue` _returnvalue "RT" (`/Game/Blueprints/Portals/BP_PortalDoorBase_2.RenderTarget` _targetportal))
              (`MaterialInstanceDynamic.SetVectorParameterValue` _returnvalue "Colour" (struct :`R` 0.671875 :`G` 0.366939 :`A` 1.0))
              (set `self.CanTeleport` true)
              (set `SceneCaptureComponent.bCaptureEveryFrame` true (`/Game/Blueprints/Portals/BP_PortalDoorBase_2.PortalView` _targetportal))
              (set `self.CanRender` true)
              (if (`self.IsTeleporting`)
                (`KismetSystemLibrary.Delay` 1.0)
                (set `self.IsTeleporting` false)
                (bind (_direction _amount) (`Timeline|OpenPortal` :!label _label_2)
                  (:`Update`
                    (`MaterialInstanceDynamic.SetScalarParameterValue` _returnvalue "Amount" _amount))
                  (:`Finished`
                    (if (xor (and (`self.CanRender`) (`self.IsOverlappingActor` (`self.CharacterRef`))) (and (`self.CanRender`) (`self.Activate`)))
                      (`PrimitiveComponent.SetCollisionEnabled` _box "QueryAndPhysics")
                      (set `self.Activate` false)
                      (set `self.RequiresActivation?` false)
                      (else
                        (`PrimitiveComponent.SetCollisionEnabled` _box "NoCollision")))))
                (else
                  (goto _label_2))))
            (:`Is Not Valid`
              (set `self.CanRender` false))))))))

(event `self.Trigger.OnComponentBeginOverlap`
  (params (OverlappedComponent :type "PrimitiveComponent Object Reference") (OtherActor :type "Actor Object Reference") (OtherComp :type "PrimitiveComponent Object Reference") (OtherBodyIndex :type Integer) (bFromSweep :type Boolean) (SweepResult :type "HitResult Structure (by ref)"))
  (bind _asbp_base_character (cast `/Game/Blueprints/Characters/BP_BaseCharacter` OtherActor))
  (`/Engine/EditorBlueprintResources/StandardMacros.IsValid` _asbp_base_character
    (:`Is Valid`
      (`KismetSystemLibrary.Delay` 0.5)
      (goto _label))))

(event `self.Trigger.OnComponentEndOverlap`
  (params (OverlappedComponent :type "PrimitiveComponent Object Reference") (OtherActor :type "Actor Object Reference") (OtherComp :type "PrimitiveComponent Object Reference") (OtherBodyIndex :type Integer))
  (bind _asbp_base_character (cast `/Game/Blueprints/Characters/BP_BaseCharacter` OtherActor))
  (`/Engine/EditorBlueprintResources/StandardMacros.IsValid` _asbp_base_character
    (:`Is Valid`
      (`KismetSystemLibrary.Delay` 1.0)
      (`/Engine/EditorBlueprintResources/StandardMacros.IsValid` (`self.TargetPortal`)
        (:`Is Valid`
          (set `self.CanTeleport` false)
          (set `self.CanRender` false)
          (set `SceneCaptureComponent.bCaptureEveryFrame` false (`/Game/Blueprints/Portals/BP_PortalDoorBase_2.PortalView` (`self.TargetPortal`)))
          (goto _label_2 :!via `Reverse`))))))

(fn `RenderPortal`
  (params (Target :type "/Game/Blueprints/Portals/BP_PortalDoorBase_2 Object Reference"))
  (bind _returnvalue (`GameplayStatics.GetPlayerCameraManager` 0))
  (bind _targetportal (`self.TargetPortal`))
  (bind _portalview (`/Game/Blueprints/Portals/BP_PortalDoorBase_2.PortalView` _targetportal))
  (`SceneComponent.K2_SetWorldLocationAndRotation` _portalview (`KismetMathLibrary.TransformLocation` (`self.GetTransform` _targetportal) (`KismetMathLibrary.InverseTransformLocation` (`KismetMathLibrary.MakeTransform` (.location (`self.GetTransform`)) (.rotation (`self.GetTransform`)) (`KismetMathLibrary.MakeVector` (* (.x (.scale (`self.GetTransform`))) -1.0) (* (.y (.scale (`self.GetTransform`))) -1.0) (.z (.scale (`self.GetTransform`))))) (`PlayerCameraManager.GetCameraLocation` _returnvalue))) (`PlayerCameraManager.GetCameraRotation` _returnvalue) false false)
  (set `SceneCaptureComponent2D.ClipPlaneBase` (`self.K2_GetActorLocation` _targetportal) _portalview)
  (set `SceneCaptureComponent2D.ClipPlaneNormal` (`self.GetActorForwardVector` _targetportal) _portalview))

(fn `TeleportToPortal`
  (params (Actor :type "Actor Object Reference") (Target :type "Actor Object Reference"))
  (returns (Teleported :type Boolean))
  (`/Engine/EditorBlueprintResources/StandardMacros.IsValid` Target
    (:`Is Valid`
      (set `/Game/Blueprints/Portals/BP_PortalDoorBase_2.IsTeleporting` true (`self.TargetPortal`))
      (bind (_sweephitresult _returnvalue) (`self.K2_SetActorLocationAndRotation` Actor (`KismetMathLibrary.MakeVector` (.x (`self.K2_GetActorLocation` Target)) (.y (`self.K2_GetActorLocation` Target)) (+ (.z (`self.K2_GetActorLocation` Target)) (`CapsuleComponent.GetUnscaledCapsuleHalfHeight` (`Character.CapsuleComponent` (cast `/Game/Blueprints/Characters/BP_BaseCharacter` Actor :!pure true))))) (`self.K2_GetActorRotation` Target) false true))
      (return _returnvalue))))

(fn `UserConstructionScript`)