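; Portal door that teleports overlapping actors to a linked BP_PortalDoor2 and spawns a BP_LevelLoader on BeginPlay.
; Tick finds the target by PortalID, and a looping timer offsets the target's PortalView from the player camera and updates its clip plane.
; Teleporting flags the target as busy and sets player 0's control rotation to the target's.
; The door destroys itself when an overlap ends after teleporting.
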(event `self.ReceiveBeginPlay`
  (`|SpawnActorFromClass` "/Game/Blueprints/BP_LevelLoader.BP_LevelLoader_C" (`self.GetTransform`) "Undefined" "OverrideRootScale" null null)
  (`KismetSystemLibrary.K2_SetTimer` null "RenderPortal" 0.001 true))

(event `self.Box.OnComponentBeginOverlap`
  (params (OverlappedComponent :type "PrimitiveComponent Object Reference") (OtherActor :type "Actor Object Reference") (OtherComp :type "PrimitiveComponent Object Reference") (OtherBodyIndex :type Integer) (bFromSweep :type Boolean) (SweepResult :type "HitResult Structure (by ref)"))
  (`self.PortalTeleport` OtherActor))

(event `PortalTeleport`
  (params (Actor :type "Actor Object Reference"))
  (if (`self.IsTeleporting`)
    (`KismetSystemLibrary.Delay` 2.0)
    (set `self.IsTeleporting` false)
    (set `self.Teleported` false)
    (else
      (`self.TeleportToPortal` Actor)
      (set `self.IsTeleporting` true)
      (set `self.Teleported` true))))

(event `self.Box.OnComponentEndOverlap`
  (params (OverlappedComponent :type "PrimitiveComponent Object Reference") (OtherActor :type "Actor Object Reference") (OtherComp :type "PrimitiveComponent Object Reference") (OtherBodyIndex :type Integer))
  (if (`self.Teleported`)
    (`self.K2_DestroyActor`)))

(event `self.ReceiveTick`
  (params (DeltaSeconds :type "Float (single-precision)"))
  ;[1 1 1] Search for a portal to teleport to
  (bind _outactors (`GameplayStatics.GetAllActorsOfClass` (`self.PortalClass`)))
  (bind _asbp_portal_door_2 (cast `/Game/Blueprints/Portals/BP_PortalDoor2` (`|GetArrayItem` _outactors (`self.PortalID`))))
  (`/Engine/EditorBlueprintResources/StandardMacros.IsValid` _asbp_portal_door_2
    (:`Is Valid`
      (set `self.TargetPortal` _asbp_portal_door_2))))

(fn `RenderPortal`
  (bind _targetportal (`self.TargetPortal`))
  (bind _returnvalue (`self.K2_GetActorLocation` _targetportal))
  (bind _portalview (`/Game/Blueprints/Portals/BP_PortalDoor2.PortalView` _targetportal))
  (bind _transformcomponent (`PlayerCameraManager.TransformComponent` (`PlayerController.PlayerCameraManager` (`GameplayStatics.GetPlayerController` 0))))
  (`/Engine/EditorBlueprintResources/StandardMacros.IsValid` _targetportal
    (:`Is Valid`
      (`SceneComponent.K2_SetWorldLocationAndRotation` _portalview (+ (- _returnvalue (`self.K2_GetActorLocation`)) (`SceneComponent.K2_GetComponentLocation` _transformcomponent)) (`SceneComponent.K2_GetComponentRotation` _transformcomponent) false true)
      (set `SceneCaptureComponent2D.ClipPlaneBase` _returnvalue _portalview)
      (set `SceneCaptureComponent2D.ClipPlaneNormal` (`self.K2_GetActorLocation`) _portalview))))

(fn `TeleportToPortal`
  (params (Actor :type "Actor Object Reference"))
  (bind _targetportal (`self.TargetPortal`))
  (bind _returnvalue (`self.K2_GetActorRotation` _targetportal))
  (`/Engine/EditorBlueprintResources/StandardMacros.IsValid` _targetportal
    (:`Is Valid`
      (set `/Game/Blueprints/Portals/BP_PortalDoor2.IsTeleporting` true _targetportal)
      (`self.K2_TeleportTo` Actor (`self.K2_GetActorLocation` _targetportal) _returnvalue)
      (`Controller.SetControlRotation` (`Pawn.GetController` (`GameplayStatics.GetPlayerCharacter` 0)) _returnvalue))))

(fn `UserConstructionScript`)