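; Portal door that pairs with a BP_PortalDoor2 found by PortalID, showing a live view through it and teleporting overlapping actors there.
; A character entering Trigger plays a timeline that opens the portal material and enables the teleport Box; leaving reverses it.
; While open, Tick mirrors the player camera onto the target's clipped scene capture, toggling capture by camera side.
; The door destroys itself on Box exit while CanTeleport is set.
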(event `self.ReceiveBeginPlay`
  (`PrimitiveComponent.SetCollisionEnabled` (`self.Box`) "NoCollision")
  (`PrimitiveComponent.SetCollisionEnabled` (`self.Trigger`) "NoCollision"))

(event `self.Box.OnComponentBeginOverlap`
  (params (OverlappedComponent :type "PrimitiveComponent Object Reference") (OtherActor :type "Actor Object Reference") (OtherComp :type "PrimitiveComponent Object Reference") (OtherBodyIndex :type Integer) (bFromSweep :type Boolean) (SweepResult :type "HitResult Structure (by ref)"))
  (if (`self.CanRender`)
    (`self.PortalTeleport` OtherActor)))

(event `PortalTeleport`
  (params (Actor :type "Actor Object Reference"))
  (if (`self.IsTeleporting`)
    (`KismetSystemLibrary.Delay` 2.0)
    (set `self.IsTeleporting` false)
    (set `self.CanTeleport` false)
    (else
      (bind _teleported (`self.TeleportToPortal` Actor))
      (set `self.IsTeleporting` true)
      (set `self.CanTeleport` _teleported))))

(event `self.Box.OnComponentEndOverlap`
  (params (OverlappedComponent :type "PrimitiveComponent Object Reference") (OtherActor :type "Actor Object Reference") (OtherComp :type "PrimitiveComponent Object Reference") (OtherBodyIndex :type Integer))
  (if (`self.CanTeleport`)
    (`self.K2_DestroyActor`)))

(event `self.ReceiveTick`
  (params (DeltaSeconds :type "Float (single-precision)"))
  (bind _targetportal (`self.TargetPortal`))
  ;[1 1 1] Search for a portal to teleport to
  (`/Engine/EditorBlueprintResources/StandardMacros.IsValid` _targetportal
    (:`Is Valid`
      (`PrimitiveComponent.SetCollisionEnabled` (`self.Trigger`) "QueryOnly")
      (if (`self.CanRender`)
        (`self.RenderPortal` _targetportal)))
    (:`Is Not Valid`
      (bind _outactors (`GameplayStatics.GetAllActorsOfClass` (`self.PortalClass`)))
      (bind _asbp_portal_door_2 (cast `/Game/Blueprints/Portals/OldPortals/BP_PortalDoor2` (`|GetArrayItem` _outactors (`self.PortalID`))))
      (`/Engine/EditorBlueprintResources/StandardMacros.IsValid` _asbp_portal_door_2
        (:`Is Valid`
          (set `self.TargetPortal` _asbp_portal_door_2)
          (`KismetSystemLibrary.Delay` 1.0))))))

(event `self.Trigger.OnComponentBeginOverlap`
  (params (OverlappedComponent :type "PrimitiveComponent Object Reference") (OtherActor :type "Actor Object Reference") (OtherComp :type "PrimitiveComponent Object Reference") (OtherBodyIndex :type Integer) (bFromSweep :type Boolean) (SweepResult :type "HitResult Structure (by ref)"))
  (bind _box (`self.Box`))
  (bind _asbp_base_character (cast `/Game/Blueprints/Characters/BP_BaseCharacter` OtherActor))
  (`/Engine/EditorBlueprintResources/StandardMacros.IsValid` _asbp_base_character
    (:`Is Valid`
      (`KismetSystemLibrary.Delay` 0.5)
      (`/Engine/EditorBlueprintResources/StandardMacros.IsValid` (`self.TargetPortal`)
        (:`Is Valid`
          (bind _returnvalue (`PrimitiveComponent.CreateDynamicMaterialInstance` (`self.Frame`) 1 "/Game/Materials/M_PortalEffect_2_Inst.M_PortalEffect_2_Inst"))
          (`MaterialInstanceDynamic.SetTextureParameterValue` _returnvalue "RT" (`/Game/Blueprints/Portals/OldPortals/BP_PortalDoor2.RenderTarget` (`self.TargetPortal`)))
          (`MaterialInstanceDynamic.SetVectorParameterValue` _returnvalue "Colour" (struct :`R` 0.671875 :`G` 0.366939 :`A` 1.0))
          (set `self.CanTeleport` true)
          (bind (_direction _amount) (`Timeline|OpenPortal` :!label _label)
            (:`Update`
              (`MaterialInstanceDynamic.SetScalarParameterValue` _returnvalue "Amount" _amount)
              (set `self.CanRender` true))
            (:`Finished`
              (if (`self.CanTeleport`)
                (`PrimitiveComponent.SetCollisionEnabled` _box "QueryAndPhysics")
                (set `self.CanTeleport` true)
                (else
                  (`PrimitiveComponent.SetCollisionEnabled` _box "NoCollision"))))))
        (:`Is Not Valid`
          (set `self.CanRender` false))))))

(event `self.Trigger.OnComponentEndOverlap`
  (params (OverlappedComponent :type "PrimitiveComponent Object Reference") (OtherActor :type "Actor Object Reference") (OtherComp :type "PrimitiveComponent Object Reference") (OtherBodyIndex :type Integer))
  (bind _asbp_base_character (cast `/Game/Blueprints/Characters/BP_BaseCharacter` OtherActor))
  (`/Engine/EditorBlueprintResources/StandardMacros.IsValid` _asbp_base_character
    (:`Is Valid`
      (`KismetSystemLibrary.Delay` 1.0)
      (set `self.CanTeleport` false)
      (set `self.CanRender` false)
      (goto _label :!via `Reverse`))))

(fn `RenderPortal`
  (params (Target :type "/Game/Blueprints/Portals/OldPortals/BP_PortalDoor2 Object Reference"))
  (bind _returnvalue (`GameplayStatics.GetPlayerCameraManager` 0))
  (bind _targetportal (`self.TargetPortal`))
  (bind _returnvalue_2 (`self.GetActorForwardVector` _targetportal))
  (bind _portalview (`/Game/Blueprints/Portals/OldPortals/BP_PortalDoor2.PortalView` _targetportal))
  (`SceneComponent.K2_SetWorldLocationAndRotation` _portalview (`KismetMathLibrary.TransformLocation` (`self.GetTransform` (`self.TargetPortal`)) (`KismetMathLibrary.InverseTransformLocation` (`KismetMathLibrary.MakeTransform` (.location (`self.GetTransform`)) (.rotation (`self.GetTransform`)) (`KismetMathLibrary.MakeVector` (* (.x (.scale (`self.GetTransform`))) -1.0) (* (.y (.scale (`self.GetTransform`))) -1.0) (.z (.scale (`self.GetTransform`))))) (`PlayerCameraManager.GetCameraLocation` _returnvalue))) (`PlayerCameraManager.GetCameraRotation` _returnvalue) false false)
  (set `SceneCaptureComponent2D.ClipPlaneBase` (`self.K2_GetActorLocation` _targetportal) _portalview)
  (set `SceneCaptureComponent2D.ClipPlaneNormal` _returnvalue_2 _portalview)
  (if (<= (`KismetMathLibrary.Dot_VectorVector` (- (`SceneComponent.K2_GetComponentLocation` (`PlayerCameraManager.TransformComponent` _returnvalue)) (`self.K2_GetActorLocation`)) _returnvalue_2) 0.0)
    (set `SceneCaptureComponent.bCaptureEveryFrame` true _portalview)
    (else
      (set `SceneCaptureComponent.bCaptureEveryFrame` false _portalview))))

(fn `TeleportToPortal`
  (params (Actor :type "Actor Object Reference"))
  (returns (Teleported :type Boolean))
  (bind _targetportal (`self.TargetPortal`))
  (`/Engine/EditorBlueprintResources/StandardMacros.IsValid` _targetportal
    (:`Is Valid`
      (set `/Game/Blueprints/Portals/OldPortals/BP_PortalDoor2.IsTeleporting` true _targetportal)
      (bind _returnvalue (`self.K2_TeleportTo` Actor (`self.K2_GetActorLocation` _targetportal) (`self.K2_GetActorRotation` _targetportal)))
      (return _returnvalue))))

(fn `UserConstructionScript`
  (bind _returnvalue (`GameUserSettings.GetGameUserSettings`))
  (bind (_returnvalue_x _returnvalue_y) (break `IntPoint` (`GameUserSettings.GetDesktopResolution` _returnvalue)))
  (bind _returnvalue_2 (`KismetRenderingLibrary.CreateRenderTarget2D` _returnvalue_x _returnvalue_y))
  (bind _output_get (set `self.RenderTarget` _returnvalue_2))
  (set `SceneCaptureComponent2D.TextureTarget` _output_get (`self.PortalView`)))