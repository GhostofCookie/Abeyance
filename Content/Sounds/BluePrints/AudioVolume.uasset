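; AudioVolume is a trigger actor that plays its Audio component while a BP_BaseCharacter is inside the Limit component and stops it on exit.
; First entry plays from zero; later entries start from the saved CurrentPlayTime.
; Playback-percent updates compute that time through a gate closed on exit.
; A DoOnce, reset on re-entry, opens the gate and adjusts the PreviousPlayTime offset once the sound's duration is exceeded.
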(event `self.Limit.OnComponentBeginOverlap`
  (params (OverlappedComponent :type "PrimitiveComponent Object Reference") (OtherActor :type "Actor Object Reference") (OtherComp :type "PrimitiveComponent Object Reference") (OtherBodyIndex :type Integer) (bFromSweep :type Boolean) (SweepResult :type "HitResult Structure (by ref)"))
  (bind _audio (`self.Audio`))
  (cast `/Game/Blueprints/Characters/BP_BaseCharacter` OtherActor)
  (if (`self.FirstTime`)
    ;[1 1 1] If it's the first time, start from zero.
    (`AudioComponent.Play` _audio 0.0)
    (set `self.FirstTime` false)
    (else
      (`AudioComponent.Play` _audio (`self.CurrentPlayTime`))
      (goto _label :!via `Reset`))))

(event `self.Limit.OnComponentEndOverlap`
  (params (OverlappedComponent :type "PrimitiveComponent Object Reference") (OtherActor :type "Actor Object Reference") (OtherComp :type "PrimitiveComponent Object Reference") (OtherBodyIndex :type Integer))
  (cast `/Game/Blueprints/Characters/BP_BaseCharacter` OtherActor)
  (`AudioComponent.Stop` (`self.Audio`))
  (goto _label_2 :!via `Close`))

(event `self.Audio.OnAudioPlaybackPercent`
  (params (PlayingSoundWave :type "SoundWave Object Reference") (PlaybackPercent :type "Float (single-precision)"))
  (`|ExecutionSequence`
    (:`then_0`
      (`/Engine/EditorBlueprintResources/StandardMacros.DoOnce` false :!label _label
        (:`Completed`
          ;[1 1 1] If the sample is finished, start over
          (if (>= (`self.CurrentPlayTime`) (`SoundBase.Duration` PlayingSoundWave))
            (set `self.PreviousPlayTime` (- (`self.CurrentPlayTime`) (`SoundBase.Duration` PlayingSoundWave)))
            (goto _label_2 :!via `Open`)
            (else
              (set `self.PreviousPlayTime` (`self.PreviousPlayTime`))
              (goto _label_2 :!via `Open`))))))
    (:`then_1`
      ;[1 1 1] Get the CurrentPlayTime in seconds.
      (`/Engine/EditorBlueprintResources/StandardMacros.Gate` true :!label _label_2
        (:`Exit`
          (set `self.CurrentPlayTime` (+ (/ (* (`SoundBase.Duration` PlayingSoundWave) (* PlaybackPercent 100.0)) 1.0) (`self.PreviousPlayTime`))))))))

(fn `UserConstructionScript`)